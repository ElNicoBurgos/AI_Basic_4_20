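; Player character Blueprint whose only live logic sets an IsFire flag while Fire or Fire2 is held.
; A disconnected shooting prototype multi-line-traces forward from Cam, lowering DanioTotal by each ParedBP's absorption and subtracting what remains from EnemyBP Vida.
; That trace chain and its damage reset never run, and the extra functions, collapsed graphs and macro are empty or unused stubs.
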(event EventBeginPlay)

(event Input|ActionEvents|InputActionFire
  (params (Key :type Key%20Structure))
  (:Pressed
    (Variables|Default|SetisFire true))
  (:Released
    (Variables|Default|SetisFire false)))

(event Input|ActionEvents|InputActionFire2
  (params (Key :type Key%20Structure))
  (:Pressed
    (Variables|Default|SetisFire true))
  (:Released
    (Variables|Default|SetisFire false)))

(fn ConstructionScript)

(fn NewFunction0
  (params (TargetArray :type Array%20of%20Hit%20Result%20Structures)))

(fn NewFunction1
  (params (TargetArray :type Array%20of%20Hit%20Result%20Structures)))